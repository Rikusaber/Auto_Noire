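; BP_NPC is a non-player character that shows its dialogue lines one at a time as floating text.
; Each DialogueInteract call advances CurrentIndex, destroys the previous BP_FloatingText and spawns a new one at the capsule's transform with the next Dialogues entry.
; Past the last line, it destroys the just-spawned text and resets the index to -1, so the following interaction restarts the conversation.
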(event EventBeginPlay)

(event Collision|EventActorBeginOverlap
  (params (OtherActor :type Actor%20Object%20Reference)))

(event EventTick
  (params (DeltaSeconds :type Float%20%28single-precision%29)))

(fn ConstructionScript)

(fn DialogueInteract
  (bind _dialogues (Variables|Default|GetDialogues))
  (Math|Integer|IncrementInt (Variables|Default|GetCurrentIndex)
    (:%20%20
      (Utilities|IsValid (Variables|Default|GetFloatingTextCurrent)
        (:Is%20Valid
          (Actor|DestroyActor (Variables|Default|GetFloatingTextCurrent)))
        (:Is%20Not%20Valid
          _))
      (bind _returnvalue (Game|SpawnActorfromClass "/Game/BPs/BP_FloatingText.BP_FloatingText_C" (Transformation|GetWorldTransform (Variables|Collision|GetCapsuleComponent)) "Undefined" 0 0))
      (bind _output_get (Variables|Default|SetFloatingTextCurrent _returnvalue))
      (if (Utilities|Array|IsValidIndex _dialogues (Variables|Default|GetCurrentIndex))
        (Rendering|Components|TextRender|SetText (Variables|/Game/BPs/BP_FloatingText.BP_FloatingText_C|GetText _returnvalue) (Utilities|Array|Get(acopy) _dialogues (Variables|Default|GetCurrentIndex)))
        (else
          (Actor|DestroyActor _output_get)
          (Variables|Default|SetCurrentIndex -1))))))